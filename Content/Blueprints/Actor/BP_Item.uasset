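; BP_Item is a world pickup actor that offers its item data to the player character's inventory on overlap.
; On BeginPlay it replaces ItemData with a newly constructed object of the same class, copying over Info so each pickup holds its own instance.
; Overlap with BP_ThirdPersonCharacter passes that object to AddItemToInventory, and the actor destroys itself only when the call returns false.
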(event `self.ReceiveActorBeginOverlap`
  (params (OtherActor :type "Actor Object Reference"))
  (if (`GameplayStatics.ObjectIsA` OtherActor "/Script/Engine.Character")
    (bind _asbp_third_person_character (cast `/Game/Blueprints/BP_ThirdPersonCharacter` OtherActor))
    (bind _returnvalue (`InventoryComponent.AddItemToInventory` (`/Game/Blueprints/BP_ThirdPersonCharacter.Inventory` _asbp_third_person_character) (`self.Item Data`)))
    (if (not _returnvalue)
      (`self.K2_DestroyActor`))))

(event `self.ReceiveBeginPlay`
  (bind _item_data (`self.Item Data`))
  (bind _returnvalue (`|GenericCreateObject` (`GameplayStatics.GetObjectClass` _item_data)))
  (`ItemData.SetInfo` _returnvalue (`ItemData.Info` _item_data))
  (set `self.Item Data` _returnvalue))

(fn `UserConstructionScript`)